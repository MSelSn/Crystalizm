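; Turtle shell boss enemy for the final fight: plays boss music, attacks nearby pawns, and spawns the slime boss when it dies.
; A looping timer sphere-traces for targets to damage, otherwise a wider trace finds the hero, widens the camera FOV and shows the boss health bar.
; Health, hit reactions and death route through BPCDamageSystem; death stops music, restores FOV and removes the bar.
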(event `self.ReceiveBeginPlay`
  (bind _returnvalue (`GameplayStatics.SpawnSound2D` "/Game/Sounds/Final/FinalFight.FinalFight" 0.5 1.0 0.0 null))
  ;[1 1 1] Attack
  (set `self.FinalSound` _returnvalue)
  (`KismetSystemLibrary.K2_SetTimerDelegate` (delegate `Attack`) 2.0 true)
  (if (not (`self.IsWidgetVisible?`))
    (bind _returnvalue_2 (`|CreateWidget` "/Game/DamageSystem/HealthBar/Enemies/WB_Enemy_HealthBar_TS_Boss.WB_Enemy_HealthBar_TS_Boss_C" null self))))

(event `Attack`
  (bind _returnvalue (`self.K2_GetActorLocation`))
  (bind _returnvalue_2 (`self.K2_GetActorLocation`))
  (bind _mesh (`self.Mesh`))
  ;[1 1 1] Attack
  (if (not (`/Game/DamageSystem/BPC_DamageSystem.IsDead` (`self.BPC_DamageSystem`)))
    (bind _outactors (`GameplayStatics.GetAllActorsWithTag` "Enemy"))
    (bind (_outhit _returnvalue_3) (`KismetSystemLibrary.SphereTraceSingleForObjects` _returnvalue (+ _returnvalue (* (`self.GetActorForwardVector`) 50.0)) 500.0 (`|MakeArray` "ObjectTypeQuery3" :!type "EObjectTypeQuery Enum") false _outactors "None" true (struct :`R` 0.052083 :`G` 1.0 :`B` 1.0 :`A` 1.0) (struct :`R` 0.747128 :`G` 1.0 :`B` 0.113053 :`A` 1.0) 0.0))
    (if _returnvalue_3
      (bind _wasdamaged (message `/Game/DamageSystem/BPI_Damagable.TakeDamage` (`.HitActor` (`GameplayStatics.BreakHitResult` _outhit)) (make `/Game/DamageSystem/S_DamageInfo` 10.0 "NewEnumerator1" "NewEnumerator1")))
      (if _wasdamaged
        (`|PlayMontage` _mesh "/Game/Characters/Enemies/Animation/TurtleShell/Attack/TurtleShell_Attack01_ANIM_Montage.TurtleShell_Attack01_ANIM_Montage")
        (else
          (`|PlayMontage` _mesh "/Game/Characters/Enemies/Animation/TurtleShell/Victory/TurtleShell_Victory_ANIM_Montage.TurtleShell_Victory_ANIM_Montage")))
      (else
        (bind _outhit_2 (`KismetSystemLibrary.SphereTraceSingleForObjects` :`Start` _returnvalue_2 :`End` _returnvalue_2 :`Radius` 1800.0 :`ObjectTypes` (`|MakeArray` "ObjectTypeQuery3" :!type "EObjectTypeQuery Enum") :`TraceColor` (struct :`R` 1.0 :`B` 0.11875 :`A` 1.0) :`TraceHitColor` (struct :`R` 0.023822 :`B` 1.0 :`A` 1.0) :`DrawTime` 5000.0 :!label _label))
        (bind _asbp_tiny_hero (cast `/Game/Characters/TinyHero/TinyHeroBP/BP_TinyHero` (`.HitActor` (`GameplayStatics.BreakHitResult` _outhit_2))))
        (`CameraComponent.SetFieldOfView` (`/Game/Characters/TinyHero/TinyHeroBP/BP_TinyHero.FollowCamera` _asbp_tiny_hero) 120.0)
        (`UserWidget.AddToViewport` (stale `self.ReceiveBeginPlay` _returnvalue_2) 0)))))

(event `DamageResponse`
  (params (DamageResponse :type "/Game/DamageSystem/E_DamageResponse Enum" :default "NewEnumerator0"))
  ;[1 1 1] Get Hit Animation
  (switch `/Game/DamageSystem/E_DamageResponse` DamageResponse
    (:`NewEnumerator1`
      (`|PlayMontage` (`self.Mesh`) "/Game/Characters/Enemies/Animation/TurtleShell/Hit-Mee/TurtleShell_GetHit_ANIM_Montage.TurtleShell_GetHit_ANIM_Montage"
        (:`then`
          (goto _label))))))

(event `Death`
  ;[1 1 1] Dying
  (`AudioComponent.Stop` (`self.FinalSound`))
  (`|PlayMontage` (`self.Mesh`) "/Game/Characters/Enemies/Animation/TurtleShell/Die/TurtleShell_Die_ANIM_Montage.TurtleShell_Die_ANIM_Montage" 0.5
    (:`then`
      (`KismetSystemLibrary.Delay` 2.0)
      (`self.K2_DestroyActor`)
      (bind _asbp_tiny_hero (cast `/Game/Characters/TinyHero/TinyHeroBP/BP_TinyHero` (`GameplayStatics.GetPlayerCharacter` 0)))
      (`CameraComponent.SetFieldOfView` (`/Game/Characters/TinyHero/TinyHeroBP/BP_TinyHero.FollowCamera` _asbp_tiny_hero) 90.0)
      (`Widget.RemoveFromParent` (stale `self.ReceiveBeginPlay` _returnvalue_2))
      (`|SpawnActorFromClass` "/Game/Maps/Final/Bosses/BP_Slime_Boss.BP_Slime_Boss_C" (`KismetMathLibrary.MakeTransform` (951.887696 -987.513686 544.589188) (struct :`Yaw` 180.0)) "AdjustIfPossibleButAlwaysSpawn" "MultiplyWithRoot" null null))))

(fn `GetCurrentHealth`
  (returns (Health :type "Float (double-precision)"))
  (return (`/Game/DamageSystem/BPC_DamageSystem.Health` (`self.BPC_DamageSystem`))))

(fn `GetMaxHealth`
  (returns (MaxHealth :type "Float (double-precision)"))
  (return (`/Game/DamageSystem/BPC_DamageSystem.MaxHealth` (`self.BPC_DamageSystem`))))

(fn `Heal`
  (params (Amount :type "Float (double-precision)"))
  (returns (NewHealth :type "Float (double-precision)"))
  (bind _newhealth (`/Game/DamageSystem/BPC_DamageSystem.Heal` (`self.BPC_DamageSystem`) Amount))
  (return _newhealth))

(fn `TakeDamage`
  (params (DamageInfo :type "/Game/DamageSystem/S_DamageInfo Structure"))
  (returns (WasDamaged :type Boolean))
  (bind _wasdamaged (`/Game/DamageSystem/BPC_DamageSystem.TakeDamage` (`self.BPC_DamageSystem`) DamageInfo))
  (return _wasdamaged))

(fn `UserConstructionScript`
  (bind _bpc_damagesystem (`self.BPC_DamageSystem`))
  (add `/Game/DamageSystem/BPC_DamageSystem.OnDeath` _bpc_damagesystem (`|CreateDelegate` :!event `Death`))
  (add `/Game/DamageSystem/BPC_DamageSystem.OnDamageResponse` _bpc_damagesystem (`|CreateDelegate` :!event `DamageResponse`)))