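; BP_Crystal is a collectable crystal that BP_TinyHero picks up by touching its box collider.
; On overlap it increments the hero's crystal counter, plays a collect sound and destroys itself.
; When the counter reaches eleven, it pauses the game, disables player input, shows the mouse cursor and displays the WB_Level_GG_Completed widget, ending the level.
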(event `self.Box.OnComponentBeginOverlap`
  (params (OverlappedComponent :type "PrimitiveComponent Object Reference") (OtherActor :type "Actor Object Reference") (OtherComp :type "PrimitiveComponent Object Reference") (OtherBodyIndex :type Integer) (bFromSweep :type Boolean) (SweepResult :type "HitResult Structure (by ref)"))
  (bind _asbp_tiny_hero (cast `/Game/Characters/TinyHero/TinyHeroBP/BP_TinyHero` OtherActor))
  (bind _crystalcountergg (`/Game/Characters/TinyHero/TinyHeroBP/BP_TinyHero.CrystalCounterGG` _asbp_tiny_hero))
  (set `/Game/Characters/TinyHero/TinyHeroBP/BP_TinyHero.CrystalCounterGG` (+ _crystalcountergg 1) _asbp_tiny_hero)
  (`GameplayStatics.PlaySound2D` "/Game/Sounds/Crystal/Crystal_Collect.Crystal_Collect" 1.0 1.0 0.0 null null)
  (`self.K2_DestroyActor`)
  (if (== _crystalcountergg 11)
    (bind _asbp_tiny_hero_2 (cast `/Game/Characters/TinyHero/TinyHeroBP/BP_TinyHero` (`GameplayStatics.GetPlayerCharacter` 0)))
    (`GameplayStatics.SetGamePaused` true)
    (`self.DisableInput` _asbp_tiny_hero_2 null)
    (set `PlayerController.bShowMouseCursor` true (`GameplayStatics.GetPlayerController` 0))
    (bind _returnvalue (`|CreateWidget` "/Game/Collectables/Completed/CompleteGG/WB_Level_GG_Completed.WB_Level_GG_Completed_C"))
    (`UserWidget.AddToViewport` _returnvalue 0)))

(fn `UserConstructionScript`)