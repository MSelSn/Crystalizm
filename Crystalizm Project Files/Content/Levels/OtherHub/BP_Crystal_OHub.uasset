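; BP_Crystal_OHub is a collectible crystal pickup for the OtherHub level that counts toward opening a gate.
; When BP_TinyHero overlaps its Box, it increments the hero's CrystalCounterHub, plays a collect sound and destroys itself.
; The crystal that brings the count to exactly six also plays a gate-opening sound and spawns BP_DoorGate2 at a hard-coded location.
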(event `self.Box.OnComponentBeginOverlap`
  (params (OverlappedComponent :type "PrimitiveComponent Object Reference") (OtherActor :type "Actor Object Reference") (OtherComp :type "PrimitiveComponent Object Reference") (OtherBodyIndex :type Integer) (bFromSweep :type Boolean) (SweepResult :type "HitResult Structure (by ref)"))
  (bind _asbp_tiny_hero (cast `/Game/Characters/TinyHero/TinyHeroBP/BP_TinyHero` OtherActor))
  (bind _crystalcounterhub (`/Game/Characters/TinyHero/TinyHeroBP/BP_TinyHero.CrystalCounterHub` _asbp_tiny_hero))
  (set `/Game/Characters/TinyHero/TinyHeroBP/BP_TinyHero.CrystalCounterHub` (+ _crystalcounterhub 1) _asbp_tiny_hero)
  (`GameplayStatics.PlaySound2D` "/Game/Sounds/Crystal/Crystal_Collect.Crystal_Collect" 1.0 1.0 0.0 null null)
  (`self.K2_DestroyActor`)
  (if (== _crystalcounterhub 6)
    (`GameplayStatics.PlaySound2D` "/Game/Sounds/DoorGates/OpenedDoorsGate.OpenedDoorsGate" 1.0 1.0 0.0 null null)
    (bind _returnvalue (`|SpawnActorFromClass` "/Game/Maps/Hub/DoorGates/BP_DoorGate2.BP_DoorGate2_C" (`KismetMathLibrary.MakeTransform` (905.166222 2182.027825 248.443684)) "AdjustIfPossibleButAlwaysSpawn" "MultiplyWithRoot" null null))
    (set `Actor.bAutoDestroyWhenFinished` false _returnvalue)))

(fn `UserConstructionScript`)