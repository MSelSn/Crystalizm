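; Slime enemy that attacks nearby pawns on a looping timer and delegates health, damage and healing to BPCDamageSystem.
; Each tick of the timer sphere-traces while ignoring "Enemy"-tagged actors, damaging a hit pawn and playing an attack or victory montage based on the result.
; Without a target, a wider trace toggles the widget health bar.
; Component events drive hit reactions, which reveal the bar, and death animation before destruction.
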(event `self.ReceiveBeginPlay`
  ;[1 1 1] Attack
  (`SceneComponent.SetHiddenInGame` (`self.Widget`) true false)
  (`KismetSystemLibrary.K2_SetTimerDelegate` (delegate `Attack`) 2.0 true)
  (bind _returnvalue (`|CreateWidget` "/Game/DamageSystem/HealthBar/Enemies/WB_Enemy_HealthBar.WB_Enemy_HealthBar_C" null self))
  (`WidgetComponent.SetWidget` (`self.Widget`) _returnvalue))

(event `Attack`
  (bind _returnvalue (`self.K2_GetActorLocation`))
  (bind _mesh (`self.Mesh`))
  ;[1 1 1] Attack
  (if (not (`/Game/DamageSystem/BPC_DamageSystem.IsDead` (`self.BPC_DamageSystem`)))
    (bind _outactors (`GameplayStatics.GetAllActorsWithTag` "Enemy"))
    (bind (_outhit _returnvalue_2) (`KismetSystemLibrary.SphereTraceSingleForObjects` _returnvalue (+ _returnvalue (* (`self.GetActorForwardVector`) 50.0)) 100.0 (`|MakeArray` "ObjectTypeQuery3" :!type "EObjectTypeQuery Enum") false _outactors "None" true (struct :`R` 0.052083 :`G` 1.0 :`B` 1.0 :`A` 1.0) (struct :`R` 0.747128 :`G` 1.0 :`B` 0.113053 :`A` 1.0) 0.0))
    (if _returnvalue_2
      (bind _wasdamaged (message `/Game/DamageSystem/BPI_Damagable.TakeDamage` (`.HitActor` (`GameplayStatics.BreakHitResult` _outhit)) (make `/Game/DamageSystem/S_DamageInfo` 5.0 "NewEnumerator1" "NewEnumerator1")))
      (if _wasdamaged
        (`|PlayMontage` _mesh "/Game/Characters/Enemies/Animation/Slime/Attack/Slime_Attack02_ANIM_Montage.Slime_Attack02_ANIM_Montage")
        (else
          (`|PlayMontage` _mesh "/Game/Characters/Enemies/Animation/Slime/Victory/Slime_Victory_ANIM_Montage.Slime_Victory_ANIM_Montage")))
      (else
        (`self.HPTracking`)))))

(event `HPTracking`
  (bind _returnvalue (`self.K2_GetActorLocation`))
  (bind _array (`|MakeArray` "ObjectTypeQuery3" :!type "EObjectTypeQuery Enum"))
  (bind _returnvalue_2 (+ _returnvalue (* (`self.GetActorForwardVector`) 50.0)))
  ;[1 1 1] Attack
  ;;[0.276 0 0] HPTracking
  (bind (_outhit _returnvalue_3) (`KismetSystemLibrary.SphereTraceSingleForObjects` _returnvalue _returnvalue_2 600.0 _array false (stale `Attack` _outactors) "None" true (struct :`R` 1.0 :`B` 0.063894 :`A` 1.0) (struct :`R` 1.0 :`B` 0.528586 :`A` 1.0) 0.0))
  (if _returnvalue_3
    (`SceneComponent.SetHiddenInGame` (`self.Widget`) false false)
    (else
      (`KismetSystemLibrary.SphereTraceSingleForObjects` _returnvalue _returnvalue_2 1000.0 _array false (stale `Attack` _outactors) "None" true (struct :`R` 0.052083 :`G` 1.0 :`B` 1.0 :`A` 1.0) (struct :`R` 0.747128 :`G` 1.0 :`B` 0.113053 :`A` 1.0) 0.0)
      (`SceneComponent.SetHiddenInGame` (`self.Widget`) true false))))

(event `Death`
  ;[1 1 1] Dying
  (`SkeletalMeshComponent.PlayAnimation` (`self.Mesh`) "/Game/Characters/Enemies/Animation/Slime/Die/Slime_Die_ANIM.Slime_Die_ANIM" true)
  (`KismetSystemLibrary.Delay` 1.3)
  (`self.K2_DestroyActor`))

(event `DamageResponse`
  (params (DamageResponse :type "/Game/DamageSystem/E_DamageResponse Enum" :default "NewEnumerator0"))
  ;[1 1 1] Get Hit Animation
  (switch `/Game/DamageSystem/E_DamageResponse` DamageResponse
    (:`NewEnumerator1`
      (`|PlayMontage` (`self.Mesh`) "/Game/Characters/Enemies/Animation/Slime/Hit-Mee/Slime_GetHit_ANIM_Montage.Slime_GetHit_ANIM_Montage"
        (:`then`
          (`SceneComponent.SetHiddenInGame` (`self.Widget`) false false))))))

(fn `GetCurrentHealth`
  (returns (Health :type "Float (double-precision)"))
  (return (`/Game/DamageSystem/BPC_DamageSystem.Health` (`self.BPC_DamageSystem`))))

(fn `GetMaxHealth`
  (returns (MaxHealth :type "Float (double-precision)"))
  (return (`/Game/DamageSystem/BPC_DamageSystem.MaxHealth` (`self.BPC_DamageSystem`))))

(fn `Heal`
  (params (Amount :type "Float (double-precision)"))
  (returns (NewHealth :type "Float (double-precision)"))
  (bind _newhealth (`/Game/DamageSystem/BPC_DamageSystem.Heal` (`self.BPC_DamageSystem`) Amount))
  (return _newhealth))

(fn `TakeDamage`
  (params (DamageInfo :type "/Game/DamageSystem/S_DamageInfo Structure"))
  (returns (WasDamaged :type Boolean))
  (bind _wasdamaged (`/Game/DamageSystem/BPC_DamageSystem.TakeDamage` (`self.BPC_DamageSystem`) DamageInfo))
  (return _wasdamaged))

(fn `UserConstructionScript`
  (bind _bpc_damagesystem (`self.BPC_DamageSystem`))
  (add `/Game/DamageSystem/BPC_DamageSystem.OnDeath` _bpc_damagesystem (`|CreateDelegate` :!event `Death`))
  (add `/Game/DamageSystem/BPC_DamageSystem.OnDamageResponse` _bpc_damagesystem (`|CreateDelegate` :!event `DamageResponse`)))